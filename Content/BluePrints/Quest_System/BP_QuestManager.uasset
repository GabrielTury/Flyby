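; BP_QuestManager runs the level's quests one at a time until all are accomplished.
; On BeginPlay it gathers every placed BP_Quest into an array, hides them all and reveals the last element as the active quest.
; CompleteQuest pops that last entry, reveals the next or prints a completion message, then updates the score on the MyHud gauges widget.
; Collision stays enabled on hidden quests, and SetActiveQuest enables collision on the manager itself.
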(event EventBeginPlay
  (CallFunction|AddQuest)
  (for _array_element (Variables|Default|GetquestArray)
    (Rendering|SetActorHiddenInGame _array_element true)
    (Collision|SetActorEnableCollision _array_element true))
  (CallFunction|SetActiveQuest))

(event Collision|EventActorBeginOverlap
  (params (OtherActor :type Actor%20Object%20Reference)))

(event EventTick
  (params (DeltaSeconds :type Float%20%28single-precision%29)))

(fn ConstructionScript)

(fn CompleteQuest
  (bind _questarray (Variables|Default|GetquestArray))
  (bind _returnvalue (Utilities|Array|Length _questarray))
  ;[1 1 1] Remove a quest atual do array
  (Utilities|Array|RemoveIndex _questarray (- _returnvalue 1))
  (if (> _returnvalue 0)
    (CallFunction|SetActiveQuest) ; Habilita nova quest
    (else
      (Development|PrintString "All quests accomplished" true true "(R=1.000000,G=0.012087,B=0.000000,A=1.000000)" 1e+01)))
  (bind _returnvalue_2 (Actor|GetActorOfClass "/Game/Hud/MyHud.MyHud_C"))
  (bind _output_get (Variables|Default|SetmyHudAsset _returnvalue_2))
  (bind _output_get_2 (Variables|Default|SetgaugesHUD (Variables|/Game/Hud/MyHud.MyHud_C|GetgaugesWidget _output_get)))
  (Default|UpdateScore _output_get_2))

(fn AddQuest
  (bind _outactors (Actor|GetAllActorsOfClass "/Game/BluePrints/Quest_System/BP_Quest.BP_Quest_C"))
  (Variables|Default|SetquestArray _outactors))

(fn GetActiveQuest
  (bind _questarray (Variables|Default|GetquestArray))
  (return (Utilities|Array|Get(acopy) _questarray (- (Utilities|Array|Length _questarray) 1))))

(fn SetActiveQuest
  (bind _activequest (CallFunction|GetActiveQuest))
  (Rendering|SetActorHiddenInGame _activequest false)
  (Collision|SetActorEnableCollision true))