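; BP_Quest is a quest objective actor that completes when an actor tagged "Crate" overlaps it.
; On BeginPlay it caches the level's BP_QuestManager.
; On overlap it loops over overlapping actors, printing each name and testing the entering actor's tag; a match sets the objective flag, calls CompleteQuest on the manager and destroys the quest actor.
; A getter exposes the objective description.
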(event EventBeginPlay
  (bind _returnvalue (Actor|GetActorOfClass "/Game/BluePrints/Quest_System/BP_QuestManager.BP_QuestManager_C"))
  (Variables|Default|SetquestManager _returnvalue))

(event Collision|EventActorBeginOverlap
  (params (OtherActor :type Actor%20Object%20Reference))
  (for _array_element (Collision|GetOverlappingActors 0 :!class /Script/Engine.Actor)
    (Development|PrintString (Utilities|GetDisplayName _array_element) true true "(R=1.000000,G=0.791492,B=0.000000,A=1.000000)" 2e+01)
    (if (Actor|ActorHasTag OtherActor "Crate")
      (CallFunction|ObjectiveCompleted)
      (Actor|DestroyActor))))

(event EventTick
  (params (DeltaSeconds :type Float%20%28single-precision%29)))

(fn ConstructionScript)

(fn ObjectiveCompleted
  (Variables|Default|Setobjective true)
  (Development|PrintString "Objetivo completo")
  (Default|CompleteQuest (Variables|Default|GetquestManager)))

(fn GetObjectiveDescription
  (return (Variables|Default|GetobjectiveDescription)))