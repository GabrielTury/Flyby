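; Basic AI pawn that wanders the navmesh and detours to a crate when notified.
; Roam chains AI MoveTo calls to random points within MovementRadius of StartLocation, stopping on failure; BeginPlay first calls it before setting StartLocation, then draws a debug circle.
; CrateBehavior stores the crate flag and location, then starts a move there; roaming resumes after a delay whether that move succeeds or fails.
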(event Custom|Roam
  ;[1 1 1] Roam player randomly in a radius
  (if (not (Variables|Default|GetnearbyCrate))
    (Development|PrintString "roam")
    (bind _randomlocation (Class|NavigationSystemV1|GetRandomLocationinNavigableRadius (Variables|Default|GetStartLocation) (Variables|Default|GetMovement%20Radius) 0 0))
    (AI|AIMoveTo self _randomlocation 0 5e+01 false
      (:OnSuccess
        (CallFunction|Roam))
      (:OnFail
        (Development|PrintString (Utilities|String|ToString(Vector) _randomlocation))))))

(event Custom|CrateNearby
  (Development|PrintString "Moving to Crate")
  (AI|AIMoveTo self (Variables|Default|GetcrateLocation) 0 1e+02 false
    (:then
      (Variables|Default|SetnearbyCrate false))
    (:OnSuccess
      (Utilities|FlowControl|Delay 1e+01)
      (CallFunction|Roam :!label _label))
    (:OnFail
      (Utilities|FlowControl|Delay 1e+01)
      (goto _label))))

(event EventBeginPlay
  (CallFunction|Roam)
  (bind _output_get (Variables|Default|SetStartLocation (Transformation|GetActorLocation)))
  (Rendering|Debug|DrawDebugCircle _output_get (Variables|Default|GetMovement%20Radius) 50 "(R=1.000000,G=0.000000,B=0.771699,A=1.000000)" 2e+01 3.0 "0.000000,1.000000,0.000000" "1.000000,0.000000,0.000000" true))

(event Collision|EventActorBeginOverlap
  (params (OtherActor :type Actor%20Object%20Reference)))

(event EventTick
  (params (DeltaSeconds :type Float%20%28single-precision%29)))

(fn ConstructionScript)

(fn CrateBehavior
  (params (newNearbyCrate :type Boolean) (crateLocation :type Vector))
  (Variables|Default|SetnearbyCrate newNearbyCrate)
  (Variables|Default|SetcrateLocation crateLocation)
  (CallFunction|CrateNearby))