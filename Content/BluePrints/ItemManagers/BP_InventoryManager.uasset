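; BP_InventoryManager is an actor that tracks a simple crate inventory as an array used like a stack.
; SetItem appends a placeholder zero entry to CrateArray and prints the new count from GetArrayLength.
; GetItem removes the newest entry and returns true, or prints a Portuguese "no items available" message and returns false when empty.
; All logic lives in these functions, as the event graph and construction script are empty.
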(event EventBeginPlay)

(event Collision|EventActorBeginOverlap
  (params (OtherActor :type Actor%20Object%20Reference)))

(event EventTick
  (params (DeltaSeconds :type Float%20%28single-precision%29)))

(fn ConstructionScript)

(fn SetItem
  ;[1 1 1] Adiciona um actor ao array
  (Utilities|Array|Add (Variables|Default|GetcrateArray) 0)
  (bind _length (CallFunction|GetArrayLength))
  (Development|PrintString (Utilities|String|ToString(Integer) _length)))

(fn GetItem
  (bind _cratearray (Variables|Default|GetcrateArray))
  (bind _returnvalue (Utilities|Array|Length _cratearray))
  ;[1 1 1] Remove o item mais novo do array
  (if (> _returnvalue 0)
    (Utilities|Array|RemoveIndex _cratearray (- _returnvalue 1))
    (return true)
    (else
      (Development|PrintString "Sem itens Disponíveis")
      (return false))))

(fn GetArrayLength
  (return (Utilities|Array|Length (Variables|Default|GetcrateArray))))