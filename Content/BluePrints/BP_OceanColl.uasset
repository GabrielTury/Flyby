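; BP_OceanColl is an ocean collision actor that ends the game when the plane hits it.
; On Hit, it checks the other component for the "Plane" tag.
; On a match it clears all widgets, shows the GameOver_Widgets screen with the mouse cursor, pauses the game and destroys the plane actor.
; The overlap, BeginPlay and Tick events are empty.
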(event EventBeginPlay)

(event EventTick
  (params (DeltaSeconds :type Float%20%28single-precision%29)))

(event Collision|EventHit
  (params (MyComp :type Primitive%20Component%20Object%20Reference) (Other :type Actor%20Object%20Reference) (OtherComp :type Primitive%20Component%20Object%20Reference) (bSelfMoved :type Boolean) (HitLocation :type Vector :default "0, 0, 0") (HitNormal :type Vector :default "0, 0, 0") (NormalImpulse :type Vector :default "0, 0, 0") (Hit :type Hit%20Result%20Structure%20%28by%20ref%29))
  (if (Components|ComponentHasTag OtherComp "Plane")
    (Viewport|RemoveAllWidgets)
    (bind _returnvalue (UserInterface|CreateWidget "/Game/Hud/GameOver_Widgets.GameOver_Widgets_C"))
    (UserInterface|Viewport|AddtoViewport _returnvalue 0)
    (Variables|/Script/Engine.PlayerController|SetbShowMouseCursor (Game|GetPlayerController 0) true)
    (Game|SetGamePaused true)
    (Actor|DestroyActor Other)))

(event Collision|EventActorBeginOverlap
  (params (OtherActor :type Actor%20Object%20Reference)))

(fn ConstructionScript)