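; BP_InventoryManager is an inventory that stores crate objects in an array used as a last-in, first-out stack.
; SetItem appends a crate and prints the new count from GetArrayLength.
; GetItem removes and returns the newest crate, or prints a Portuguese "no items available" message when the array is empty.
; The event graph and construction script contain no logic, so all behavior runs through these functions.
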(event EventBeginPlay)

(event Collision|EventActorBeginOverlap
  (params (OtherActor :type Actor%20Object%20Reference)))

(event EventTick
  (params (DeltaSeconds :type Float%20%28single-precision%29)))

(fn ConstructionScript)

(fn SetItem
  (params (CrateObject :type BP%20Crate%20Object%20Reference))
  ;[1 1 1] Adiciona um actor ao array
  (Utilities|Array|Add (Variables|Default|GetitemArray) CrateObject)
  (bind _length (CallFunction|GetArrayLength))
  (Development|PrintString (Utilities|String|ToString(Integer) _length)))

(fn GetItem
  (bind _itemarray (Variables|Default|GetitemArray))
  (bind _returnvalue (Utilities|Array|Length _itemarray))
  (bind _returnvalue_2 (- _returnvalue 1))
  ;[1 1 1] Remove o item mais novo do array
  (if (> _returnvalue 0)
    (bind _output_get (Variables|Default|SetreturnCrate (Utilities|Array|Get(acopy) _itemarray _returnvalue_2)))
    (Utilities|Array|RemoveIndex _itemarray _returnvalue_2)
    (return _output_get)
    (else
      (Development|PrintString "Sem itens Disponíveis"))))

(fn GetArrayLength
  (return (Utilities|Array|Length (Variables|Default|GetitemArray))))